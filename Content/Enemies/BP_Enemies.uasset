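; Enemy Blueprint that grows in on spawn, chases on sight and breaks apart when hit.
; PawnSensing triggers AIMoveTo, targeting the player controller rather than its pawn.
; A looping timer from BeginPlay raises uniform scale until it reaches one, and is never cleared.
; OnHit hides the capsule hierarchy, spawns BpGcClass (likely a geometry collection) in place plus FS_master at the hit point, then destroys the enemy.
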(event OnSeePawn(PawnSensing)
  (params (Pawn :type Pawn%20Object%20Reference))
  ;[1 1 1] Follow player
  (AI|AIMoveTo self "0, 0, 0" (Game|GetPlayerController 0) 5.0 false))

(event Custom|On%20Hit
  (params (Hit%20point :type Vector))
  ;[1 1 1] On Hit
  (Rendering|SetVisibility (Variables|Collision|GetCapsuleComponent) false true)
  (bind _returnvalue (Game|SpawnActorfromClass (Variables|Default|Getbp_gc_class) (Transformation|GetActorTransform) "AlwaysSpawn" "MultiplyWithRoot" 0 0))
  (Game|SpawnActorfromClass "/Game/Enemies/Unicorn/SM_unicorn_SM_unicorn/FS_master.FS_master_C" (Math|Conversions|ToTransform(Vector) Hit%20point) "AlwaysSpawn" "MultiplyWithRoot" _returnvalue 0)
  (Actor|DestroyActor))

(event Custom|scale
  (bind _returnvalue (Transformation|GetActorTransform))
  (bind _scale (Math|Transform|BreakTransform _returnvalue))
  (bind _x (Math|Vector|BreakVector _scale))
  (bind _returnvalue_2 (+ _x 0.05))
  ;[50 50 50] Scale on start
  (Math|Float|CompareFloat _x 1.0
    (:<
      (Transformation|SetActorScale3D (Math|Vector|MakeVector _returnvalue_2 _returnvalue_2 _returnvalue_2)))))

(event EventBeginPlay
  ;[50 50 50] Scale on start
  (bind _returnvalue (Utilities|Time|SetTimerbyEvent (delegate Custom|scale) 0.01 true))
  (Variables|Default|Setscale_timer_handler _returnvalue))

(fn ConstructionScript)