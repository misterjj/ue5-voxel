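; BP_cupcake is a cupcake enemy that reacts to how close the player pawn is.
; Each Tick it checks that distance: at mid range it raises its walk speed and turns its stylized Niagara fire blue with a set lifetime, with no revert.
; At close range it calls OnHit at its own location instead.
; The construction script assigns BP_GC_cupcake as its BpGcClass.
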(event Collision|EventActorBeginOverlap
  (params (OtherActor :type Actor%20Object%20Reference)))

(event EventTick
  (params (DeltaSeconds :type Float%20%28single-precision%29))
  (bind _returnvalue (Game|Player|GetPlayerPawn 0))
  (bind _ns_stylizefire (Variables|Default|GetNS_StylizeFire))
  (bind _returnvalue_2 (Transformation|GetDistanceTo _returnvalue))
  (if (<= _returnvalue_2 4e+02)
    (if (<= _returnvalue_2 1.5e+02)
      (CallFunction|OnHit (Transformation|GetActorLocation))
      (else
        (Variables|/Script/Engine.CharacterMovementComponent|SetMaxWalkSpeed (Variables|Character|GetCharacterMovement) 5e+02)
        (Niagara|SetNiagaraVariable(LinearColor) _ns_stylizefire "USer.Color" (Utilities|Struct|MakeLinearColor 1.0 3.5 3e+01 1.0))
        (Niagara|SetNiagaraVariable(Float) _ns_stylizefire "User.LifeTime" 3.0)))))

(fn ConstructionScript
  (Variables|Default|Setbp_gc_class "/Game/Enemies/cupcake/SM_cupcake_SM_cupcake/BP_GC_cupcake.BP_GC_cupcake_C"))