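; BP_EarthSpike is a Barbarian attack actor that hits enemies it overlaps as its sphere moves.
; Actor overlaps cast to BP_Enemies and call OnHit with a point slightly above the sphere's location.
; The Moveto event waits briefly, moves the sphere along its relative X axis, then fires the OnEarthSpikeEnd dispatcher and destroys the actor.
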(event Custom|Move%20to
  ;[50 50 50] Move to
  (Utilities|FlowControl|Delay 0.4)
  (Components|MoveComponentTo (Variables|Default|GetSphere) "400.000000,0.000000,0.000000" "0, 0, 0" false false 0.2 false)
  (Default|CallOnEarthSpikeEnd)
  (Actor|DestroyActor))

(event EventBeginPlay)

(event Collision|EventActorBeginOverlap
  (params (OtherActor :type Actor%20Object%20Reference))
  ;[50 50 50] Collision
  (bind _asbp_enemies (Utilities|Casting|CastToBP_Enemies OtherActor))
  (Default|OnHit _asbp_enemies (+ (Transformation|GetWorldLocation (Variables|Default|GetSphere)) "0.000000,0.000000,100.000000")))

(event EventTick
  (params (DeltaSeconds :type Float%20%28single-precision%29)))

(fn ConstructionScript)